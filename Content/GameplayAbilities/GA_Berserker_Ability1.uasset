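; Berserker's first gameplay ability, which commits, then spawns a projectile at the caster's location and rotation, owned by the owning actor.
; It waits once for a collision gameplay event (tagged Knight.Ability1 despite the Berserker name), net-syncs with only the server waiting, then applies the damage effect to the payload's targets.
; The ability ends after that hit or when the projectile's lifespan elapses, cleaning up the event listener on end.
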(event `self.K2_ActivateAbility`
  (bind _returnvalue (`self.GetAvatarActorFromActorInfo`))
  (`self.K2_CommitAbility`)
  (bind _asplayer_character (cast `/Game/Characters/PlayerCharacter` _returnvalue))
  (bind (_asynctaskproxy _spawnedactor) (`GameplayTask_SpawnActor.SpawnActor` self (`Actor.K2_GetActorLocation` _returnvalue) (`Actor.K2_GetActorRotation` _returnvalue) "/Game/GameplayAbilities/Projectile_Berserker_Ability1.Projectile_Berserker_Ability1_C" false _returnvalue _asplayer_character)
    (:`Success`
      (set `self.Projectile` _spawnedactor)
      (`Actor.SetOwner` _spawnedactor (`self.GetOwningActorFromActorInfo`))
      (bind (_asynctaskproxy_2 _payload) (`AbilityTask_WaitGameplayEvent.WaitGameplayEvent` (struct :`TagName` "sendCollision.Knight.Ability1") null true)
        (:`then`
          (set `self.ASync` _asynctaskproxy_2)
          (`GameplayTask_WaitDelay.TaskWaitDelay` self (`Actor.GetLifeSpan` (`self.Projectile`))
            (:`OnFinish`
              (`self.K2_EndAbility`))))
        (:`EventReceived`
          (`AbilityTask_NetworkSyncPoint.WaitNetSync` "OnlyServerWait"
            (:`OnSync`
              (`self.BP_ApplyGameplayEffectToTarget` (`.TargetData` (break `GameplayEventData` _payload)) "/Game/GameplayAbilities/GE_Berserker_Ability1_Damage.GE_Berserker_Ability1_Damage_C")
              (`self.K2_EndAbility`))))))))

(event `self.K2_OnEndAbility`
  (params (bWasCancelled :type Boolean))
  (bind _async (`self.ASync`))
  (`/Engine/EditorBlueprintResources/StandardMacros.IsValid` _async
    (:`Is Valid`
      (`GameplayTask.EndTask` _async))))